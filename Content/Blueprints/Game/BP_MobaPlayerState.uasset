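; BP_MobaPlayerState is the MOBA player state that holds each player's lobby team.
; CopyProperties passes LobbyTeam to the new player state, so the team survives the handover, such as during seamless travel.
; ROS_SetLobbyTeam stores the value and relays it through MC_SetLobbyTeam, a server-then-multicast pattern going by the prefixes.
; BeginPlay and CopyProperties print the team for debugging.
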(event Custom|MC_SetLobbyTeam
  (params (Lobby%20Team :type EGameTeam%20Enum :default "Blue"))
  (Variables|Default|SetLobbyTeam Lobby%20Team))

(event Custom|ROS_SetLobbyTeam
  (params (Lobby%20Team :type EGameTeam%20Enum :default "Blue"))
  (bind _output_get (Variables|Default|SetLobbyTeam Lobby%20Team))
  (CallFunction|MCSetLobbyTeam _output_get))

(event EventBeginPlay
  (Development|PrintString (Utilities|String|EnumtoString (Variables|Default|GetLobbyTeam)) true true "(R=0.000000,G=1.000000,B=0.205096,A=1.000000)"))

(event EventTick
  (params (DeltaSeconds :type Float%20%28single-precision%29)))

(event EventCopyProperties
  (params (NewPlayerState :type Player%20State%20Object%20Reference))
  (bind _lobbyteam (Variables|Default|GetLobbyTeam))
  (|CallParentFunction NewPlayerState)
  (bind _asbp_moba_player_state (Utilities|Casting|CastToBP_MobaPlayerState NewPlayerState))
  (CallFunction|ROSSetLobbyTeam _asbp_moba_player_state _lobbyteam)
  (Development|PrintString (Utilities|String|Append (Utilities|String|EnumtoString _lobbyteam) " | " (Utilities|String|EnumtoString (Variables|/Script/MobaDegree.MobaPlayerState|GetLobbyTeam _asbp_moba_player_state)) " | CopyProperties") true true "(R=0.000000,G=0.660000,B=1.000000,A=1.000000)" 2e+02))

(fn ConstructionScript)