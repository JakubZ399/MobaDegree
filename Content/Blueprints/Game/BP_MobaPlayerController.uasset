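; BP_MobaPlayerController is the player controller for the MOBA game, handling main HUD creation and player respawn.
; On BeginPlay it calls ROC_UI, which creates the UW_MainUI widget, stores it as MainUI and adds it to the viewport.
; ROS_RequestRespawn waits a short fixed delay, then asks BP_MobaDegreeGameMode to restart this player.
; The ROC and ROS prefixes suggest client and server RPCs.
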(event Custom|ROC_UI
  (bind _returnvalue (UserInterface|CreateWidget "/Game/Blueprints/UI/Widget/UW_MainUI.UW_MainUI_C"))
  (bind _output_get (Variables|Default|SetMainUI _returnvalue))
  (UserInterface|Viewport|AddtoViewport _output_get 0))

(event Custom|ROS_RequestRespawn
  (Utilities|FlowControl|Delay 3.0)
  (bind _asbp_moba_degree_game_mode (Utilities|Casting|CastToBP_MobaDegreeGameMode (Game|GetGameMode)))
  (Class|GameModeBase|RestartPlayer _asbp_moba_degree_game_mode self))

(event EventBeginPlay
  (|CallParentFunction)
  (CallFunction|ROCUI))

(event EventTick
  (params (DeltaSeconds :type Float%20%28single-precision%29))
  (|CallParentFunction DeltaSeconds))

(fn ConstructionScript)