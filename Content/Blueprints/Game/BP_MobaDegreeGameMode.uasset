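; Game mode for a team-based MOBA that chooses where and as what each player spawns.
; FindPlayerStart sorts player starts by BlueSpawn and RedSpawn tags and picks a random one for the player's team, with untagged starts or parent logic serving teamless players.
; The pawn class comes from the player state's CharacterClass, falling back to the parent default.
; A RespawnPlayer event restarts a given player.
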(event Custom|RespawnPlayer
  (params (NewPlayer :type Controller%20Object%20Reference))
  (Class|GameModeBase|RestartPlayer NewPlayer))

(fn ConstructionScript)

(fn FindPlayerStart
  (params (Player :type Controller%20Object%20Reference) (IncomingName :type String))
  (bind _asmoba_player_state (Utilities|Casting|CastToMobaPlayerState (Variables|/Script/Engine.Controller|GetPlayerState Player)))
  (Utilities|Array|Clear (Variables|Default|GetPlayerStartBlue))
  (Utilities|Array|Clear (Variables|Default|GetPlayerStartRed))
  (bind _returnvalue (Class|TeamComponent|GetTeam (Variables|/Script/MobaDegree.MobaPlayerState|GetTeamComponent _asmoba_player_state)))
  (LocalVariables|SetTeam _returnvalue)
  (bind _outactors (Actor|GetAllActorsOfClass "/Script/Engine.PlayerStart"))
  (for _array_element _outactors
    (if (== (Variables|/Script/Engine.PlayerStart|GetPlayerStartTag _array_element) "BlueSpawn")
      (Utilities|Array|AddUnique (Variables|Default|GetPlayerStartBlue) _array_element)
      (elif (== (Variables|/Script/Engine.PlayerStart|GetPlayerStartTag _array_element) "RedSpawn")
        (Utilities|Array|AddUnique (Variables|Default|GetPlayerStartRed) _array_element)
        (else
          (Variables|Default|SetPlayerStart _array_element)))))
  (if (or (Utilities|Array|IsNotEmpty (Variables|Default|GetPlayerStartBlue)) (Utilities|Array|IsNotEmpty (Variables|Default|GetPlayerStartRed)))
    (if (Utilities|Enum|Equal(Enum) (LocalVariables|GetTeam) "Blue")
      (return (.OutItem (Utilities|Array|Random (Variables|Default|GetPlayerStartBlue))))
      (elif (Utilities|Enum|Equal(Enum) (LocalVariables|GetTeam) "Red")
        (return (.OutItem (Utilities|Array|Random (Variables|Default|GetPlayerStartRed))))
        (else
          _))))
  (if (Utilities|Enum|Equal(Enum) (LocalVariables|GetTeam) "None")
    (bind _playerstart (Variables|Default|GetPlayerStart)
      (:then
        (return _playerstart))
      (:else
        (bind _returnvalue_2 (|CallParentFunction Player IncomingName))
        (return _returnvalue_2)))))

(fn GetDefaultPawnClassforController
  (params (InController :type Controller%20Object%20Reference))
  (bind _asmoba_player_state (Utilities|Casting|CastToMobaPlayerState (Variables|/Script/Engine.Controller|GetPlayerState InController))
    (:then
      (if (Utilities|IsValidClass (Variables|/Script/MobaDegree.MobaPlayerState|GetCharacterClass _asmoba_player_state))
        (return (Variables|/Script/MobaDegree.MobaPlayerState|GetCharacterClass _asmoba_player_state))
        (else
          _)))
    (:CastFailed
      _))
  (bind _returnvalue (|CallParentFunction InController))
  (return _returnvalue))