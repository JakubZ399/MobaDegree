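; Base MOBA player character with zoomable camera, auto-attack and death/respawn, using the Gameplay Ability System.
; Authority grants the primary attack ability; Tick chases AttackTarget, then stops, faces it and fires the ability on an AttackSpeed delay.
; A depleted attribute or debug R triggers death, which requests respawn through BP_MobaPlayerController and destroys the pawn.
; Click-to-move Movement is unused, and IsInAttackRange compares distance with itself, ignoring AttackRange.
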(event Custom|Movement
  (bind _returnvalue (Game|GetPlayerController 0))
  (bind (_hitresult _returnvalue_2) (Game|Player|GetHitResultUnderCursorbyChannel _returnvalue "TraceTypeQuery1" true))
  (if _returnvalue_2
    (AI|Navigation|SimpleMovetoLocation _returnvalue (.Location (Collision|BreakHitResult _hitresult)))))

(event Custom|HandleDeath
  (CallFunction|ROSHandleDeath))

(event Custom|ROS_HandleDeath
  (bind _asbp_moba_player_controller (Utilities|Casting|CastToBP_MobaPlayerController (Pawn|GetController)))
  (Input|DisableInput 0)
  (Class|Pawn|DetachfromControllerPendingDestroy)
  (Utilities|FlowControl|Delay 0.2)
  (Default|ROSRequestRespawn _asbp_moba_player_controller)
  (Actor|DestroyActor))

(event Input|EnhancedActionEvents|EnhancedInputActionIA_Zoom
  (params (ActionValue :type Float%20%28double-precision%29) (ElapsedSeconds :type Float%20%28double-precision%29) (TriggeredSeconds :type Float%20%28double-precision%29) (InputAction :type Input%20Action%20Object%20Reference :default "/Game/Blueprints/Player/Input/Actions/IA_Zoom.IA_Zoom"))
  (bind _cameraboom (Variables|Default|GetCameraBoom))
  ;[1 1 1] Zoom
  (Variables|/Script/Engine.SpringArmComponent|SetTargetArmLength _cameraboom (Math|Float|Clamp(Float) (+ (* ActionValue -5e+02) (Variables|/Script/Engine.SpringArmComponent|GetTargetArmLength _cameraboom)) 1e+03 2e+03)))

(event EventTick
  (params (DeltaSeconds :type Float%20%28single-precision%29))
  (bind _returnvalue (Class|MobaDegreeCharacter|GetAbilitySystemComponent))
  (bind _returnvalue_2 (Transformation|GetActorLocation))
  (bind _attacktarget (Variables|Default|GetAttackTarget))
  (bind (_bfound _returnvalue_3) (Class|AbilitySystemComponent|GetGameplayAttributeValue _returnvalue "(AttributeName=\"Health\",Attribute=/Script/MobaDegree.MobaAttributeSet:Health,AttributeOwner=\"/Script/CoreUObject.Class'/Script/MobaDegree.MobaAttributeSet'\")"))
  (bind _returnvalue_4 (Transformation|GetActorLocation _attacktarget))
  (Utilities|FlowControl|Sequence
    (:then_0
      (Utilities|IsValid _returnvalue
        (:Is%20Valid
          (if (and _bfound (<= _returnvalue_3 0.0))
            (Utilities|FlowControl|DoOnce false
              (:Completed
                (CallFunction|HandleDeath)))))))
    (:then_1
      (bind _attacktarget_2 (Variables|Default|GetAttackTarget)
        (:then
          (if (< (Math|Vector|Distance2D(Vector) _returnvalue_4 _returnvalue_2) (Variables|Default|GetAttackRange))
            (Utilities|FlowControl|DoOnce false :!label _label
              (:Completed
                (Variables|Default|SetbIsAttacking true)
                (Components|Movement|StopMovementImmediately (Variables|Character|GetCharacterMovement))
                (Transformation|SetActorRotation (Math|Rotator|FindLookatRotation (Transformation|GetActorLocation) (Transformation|GetActorLocation _attacktarget_2)))
                (Abilities|TryActivateAbilitybyClass (Class|MobaDegreeCharacter|GetAbilitySystemComponent) (Variables|Default|GetGA_PrimaryAttack) true)
                (Utilities|FlowControl|Delay (Variables|Default|GetAttackSpeed))
                (goto _label Reset)))
            (else
              (Pawn|Input|AddMovementInput (- _returnvalue_4 _returnvalue_2) 1.0 false))))
        (:else)))))

(event EventBeginPlay
  (|CallParentFunction)
  (Utilities|FlowControl|Delay 1.0)
  (Networking|SwitchHasAuthority
    (:Authority
      (GameplayAbilities|GiveAbility (Class|MobaDegreeCharacter|GetAbilitySystemComponent) (Variables|Default|GetGA_PrimaryAttack) 1 -1))))

(event Input|KeyboardEvents|DebugKeyR
  (params (Key :type Key%20Structure :default "None") (ActionValue :type Input%20Action%20Value%20Structure))
  (:Pressed
    (CallFunction|HandleDeath)))

(event Input|KeyboardEvents|G
  (params (Key :type Key%20Structure :default "None")))

(fn ConstructionScript)

(fn IsinAttackRange
  (bind _attacktarget (Variables|Default|GetAttackTarget)
    (:then
      (bind _output_get (LocalVariables|SetDistance (Math|Vector|Distance(Vector) (Transformation|GetActorLocation) (Transformation|GetActorLocation _attacktarget))))
      (return (<= _output_get (Math|Vector|Distance(Vector) (Transformation|GetActorLocation) (Transformation|GetActorLocation _attacktarget)))))
    (:else
      (return false))))