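; MOBA nexus actor whose destruction ends the match by sending the server to the GameSummary level.
; Tick polls its Tower reference and destroys the linked Wall once the tower is no longer valid.
; On Destroyed it calls ServerTravel on the game mode as a listen server; win/lose handling is only a debug print, and the fetched team is unused.
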(event EventBeginPlay)

(event Collision|EventActorBeginOverlap
  (params (OtherActor :type Actor%20Object%20Reference)))

(event EventTick
  (params (DeltaSeconds :type Float%20%28single-precision%29))
  (Utilities|IsValid (Variables|Default|GetTower)
    (:Is%20Not%20Valid
      (bind _wall (Variables|Default|GetWall)
        (:then
          (Actor|DestroyActor _wall))
        (:else)))))

(event EventDestroyed
  ;[1 1 1] Add this
  (Class|TeamComponent|GetTeam (Variables|Default|GetTeamComponent))
  (bind _asbp_moba_degree_game_mode (Utilities|Casting|CastToBP_MobaDegreeGameMode (Game|GetGameMode)))
  (Class|MobaDegreeGameMode|ServerTravel _asbp_moba_degree_game_mode "/Game/Blueprints/Levels/GameSummary?listen")
  (Development|PrintString "NEXUS ADD WIN/LOSE" true true "(R=1.000000,G=0.000000,B=0.078214,A=1.000000)"))

(fn ConstructionScript
  (|CallParentFunction))