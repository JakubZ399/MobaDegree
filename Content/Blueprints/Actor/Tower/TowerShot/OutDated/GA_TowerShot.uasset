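; Gameplay ability for a MOBA tower's ranged attack, filed under OutDated, that fires a tower shot at the tower's current target.
; On activation it spawns a BP_TowerShot at the avatar tower's projectile spawner and passes it the attack component's target.
; It then ends with a debug print; the cooldown commit is disconnected, and a failed cast stops execution before EndAbility.
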(event Ability|EventActivateAbility
  ;[1 1 1] To interface
  (bind _asbp_moba_tower (Utilities|Casting|CastToBP_MobaTower (Ability|GetAvatarActorfromActorInfo)))
  (bind _returnvalue (Game|SpawnActorfromClass "/Game/Blueprints/Actor/Tower/TowerShot/BP_TowerShot.BP_TowerShot_C" (Class|MobaTower|GetProjectileSpawnerTransform _asbp_moba_tower) "Undefined" "MultiplyWithRoot" 0 0))
  ;[1 1 1] to interface
  (bind _asbp_tower_shot (Utilities|Casting|CastToBP_TowerShot _returnvalue))
  (Default|AttackTarget _asbp_tower_shot (Variables|/Script/MobaDegree.AttackComponent|GetAttackTarget (Variables|/Script/MobaDegree.MobaTower|GetAttackComponent _asbp_moba_tower)))
  (Ability|EndAbility))

(event Ability|EventOnEndAbility
  (params (bWasCancelled :type Boolean))
  (Development|PrintString "AbilityEnd" true true "(R=1.000000,G=0.000000,B=0.319261,A=1.000000)"))