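; BP_TowerShot is a tower projectile that homes in on a given target and applies a gameplay effect on hit.
; AttackTarget plays a timeline that eases the actor with a sinusoidal curve from its current location toward the target's live location on each update.
; When the sphere overlaps a BP_TopDownCharacter, its ability system applies GE_TowerShot to that character, then the shot destroys itself.
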(event OnComponentBeginOverlap(Sphere)
  (params (OverlappedComponent :type Primitive%20Component%20Object%20Reference) (OtherActor :type Actor%20Object%20Reference) (OtherComp :type Primitive%20Component%20Object%20Reference) (OtherBodyIndex :type Integer) (bFromSweep :type Boolean) (SweepResult :type Hit%20Result%20Structure%20%28by%20ref%29))
  (bind _asbp_top_down_character (Utilities|Casting|CastToBP_TopDownCharacter OtherActor))
  (GameplayEffects|ApplyGameplayEffectToTarget :self (Variables|Default|GetAbilitySystem) :GameplayEffectClass "/Game/Blueprints/Actor/Tower/GE_TowerShot.GE_TowerShot_C" :Target (Ability|GetAbilitySystemComponent _asbp_top_down_character))
  (Actor|DestroyActor))

(event Custom|AttackTarget
  (params (AttackTarget :type Actor%20Object%20Reference))
  (Variables|Default|SetAttack%20Target AttackTarget)
  (bind _attack_target (Variables|Default|GetAttack%20Target)
    (:then
      (bind _time (Timeline|Timeline Play)
        (:Update
          (Transformation|SetActorLocation (Math|Interpolation|Ease "SinusoidalInOut" _time (Transformation|GetActorLocation) (Transformation|GetActorLocation _attack_target)) false false))))
    (:else)))

(fn ConstructionScript)