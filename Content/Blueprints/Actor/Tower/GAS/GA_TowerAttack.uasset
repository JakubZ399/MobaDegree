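; Gameplay ability that makes a MOBA tower fire a shot at its current attack target.
; It plays the tower attack montage and waits for a Tower.Shoot gameplay event.
; On that event it spawns a BP_TowerShot at the muzzle socket and launches it at the AttackComponent's target, destroying it if the target is invalid.
; The ability ends after the shot, when the montage finishes or is interrupted, or if the avatar is not a tower.
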(event Ability|EventActivateAbility
  (bind _asbp_moba_tower (Utilities|Casting|CastToBP_MobaTower (Ability|GetAvatarActorfromActorInfo))
    (:then
      (bind _output_get (Variables|Default|SetBP%20Moba%20Tower _asbp_moba_tower))
      (|PlayMontageandWaitforEvent "None" "/Game/Blueprints/Actor/Tower/Animation/AM_TowerAttack.AM_TowerAttack" "(GameplayTags=((TagName=\"Tower.Shoot\")))" 1.0 "None" true 1.0
        (:OnCompleted
          (Ability|EndAbility :!label _label))
        (:OnInterrupted
          (goto _label))
        (:OnCancelled
          (goto _label))
        (:EventReceived
          (bind _returnvalue (Game|SpawnActorfromClass "/Game/Blueprints/Actor/Tower/TowerShot/BP_TowerShot.BP_TowerShot_C" (Transformation|GetSocketTransform (Class|MobaTower|GetTowerMesh _output_get) "Muzzle_01" "RTS_World") "Undefined" "MultiplyWithRoot" 0 0))
          (bind _output_get_2 (Variables|Default|SetTowerShot _returnvalue))
          (Utilities|IsValid (Variables|/Script/MobaDegree.AttackComponent|GetAttackTarget (Variables|/Script/MobaDegree.MobaTower|GetAttackComponent _asbp_moba_tower))
            (:Is%20Valid
              (Class|TowerShot|AttackTarget _output_get_2 (Variables|/Script/MobaDegree.AttackComponent|GetAttackTarget (Variables|/Script/MobaDegree.MobaTower|GetAttackComponent _asbp_moba_tower)))
              (Ability|EndAbility))
            (:Is%20Not%20Valid
              (Actor|DestroyActor _output_get_2)
              (Ability|EndAbility))))))
    (:CastFailed
      (Ability|EndAbility))))

(event Ability|EventOnEndAbility
  (params (bWasCancelled :type Boolean)))