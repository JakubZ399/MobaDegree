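; Base MOBA player character with camera zoom and auto-attack on a target, built on the Gameplay Ability System.
; On BeginPlay the server grants the primary attack ability, then writes the player state's team to a debug widget.
; Tick moves toward AttackTarget until in range, then stops, faces it and activates the hardcoded Khaimera attack behind a delay-reset DoOnce.
; A click-to-move Movement event exists, but its only call is unreachable.
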(event Custom|Movement
  (bind _returnvalue (Game|GetPlayerController 0))
  (bind (_hitresult _returnvalue_2) (Game|Player|GetHitResultUnderCursorbyChannel _returnvalue "TraceTypeQuery1" true))
  (if _returnvalue_2
    (AI|Navigation|SimpleMovetoLocation _returnvalue (.Location (Collision|BreakHitResult _hitresult)))))

(event Custom|TextDebug
  (bind _aswbp_test_text (Utilities|Casting|CastToWBP_TestText (UserInterface|GetWidget (Variables|Default|GetDEBUG%20TEAM))))
  (bind _asbp_moba_player_state (Utilities|Casting|CastToBP_MobaPlayerState (Variables|Default|GetPlayerState)))
  (bind _returnvalue (Class|TeamComponent|GetTeam (Variables|/Script/MobaDegree.MobaPlayerState|GetTeamComponent _asbp_moba_player_state)))
  (Default|SetDebugText _aswbp_test_text _returnvalue)
  (Development|PrintString (Utilities|String|Append "TeamChange: " "")))

(event Input|EnhancedActionEvents|EnhancedInputActionIA_Zoom
  (params (ActionValue :type Float%20%28double-precision%29) (ElapsedSeconds :type Float%20%28double-precision%29) (TriggeredSeconds :type Float%20%28double-precision%29) (InputAction :type Input%20Action%20Object%20Reference :default "/Game/Blueprints/Player/Input/Actions/IA_Zoom.IA_Zoom"))
  (bind _cameraboom (Variables|Default|GetCameraBoom))
  ;[1 1 1] Zoom
  (Variables|/Script/Engine.SpringArmComponent|SetTargetArmLength _cameraboom (Math|Float|Clamp(Float) (+ (* ActionValue -5e+02) (Variables|/Script/Engine.SpringArmComponent|GetTargetArmLength _cameraboom)) 1e+03 4e+03)))

(event EventTick
  (params (DeltaSeconds :type Float%20%28single-precision%29))
  (bind _returnvalue (Transformation|GetActorLocation))
  (bind _attacktarget (Variables|Default|GetAttackTarget))
  (bind _returnvalue_2 (Transformation|GetActorLocation _attacktarget))
  (bind _attacktarget_2 (Variables|Default|GetAttackTarget)
    (:then
      (if (< (Math|Vector|Distance2D(Vector) _returnvalue_2 _returnvalue) (Variables|Default|GetAttackRange))
        (Utilities|FlowControl|DoOnce false :!label _label
          (:Completed
            (Variables|Default|SetbIsAttacking true)
            (Components|Movement|StopMovementImmediately (Variables|Character|GetCharacterMovement))
            (Transformation|SetActorRotation (Math|Rotator|FindLookatRotation (Transformation|GetActorLocation) (Transformation|GetActorLocation _attacktarget_2)))
            (Abilities|TryActivateAbilitybyClass (Class|MobaDegreeCharacter|GetAbilitySystemComponent) "/Game/Blueprints/Player/Characters/Khaimera/GAS/GA_KhaimeraAttack.GA_KhaimeraAttack_C" true)
            (Utilities|FlowControl|Delay 2.0)
            (goto _label Reset)))
        (else
          (Pawn|Input|AddMovementInput (- _returnvalue_2 _returnvalue) 1.0 false))))
    (:else)))

(event EventBeginPlay
  (Utilities|FlowControl|Delay 1.0)
  (Networking|SwitchHasAuthority
    (:Authority
      (GameplayAbilities|GiveAbility (Class|MobaDegreeCharacter|GetAbilitySystemComponent) (Variables|Default|GetGA_PrimaryAttack) 1 -1)
      (Utilities|FlowControl|Delay 1.0)
      (bind _aswbp_test_text (Utilities|Casting|CastToWBP_TestText (UserInterface|GetWidget (Variables|Default|GetDEBUG%20TEAM))))
      (bind _asbp_moba_player_state (Utilities|Casting|CastToBP_MobaPlayerState (Variables|Default|GetPlayerState)))
      (bind _returnvalue (Class|TeamComponent|GetTeam (Variables|/Script/MobaDegree.MobaPlayerState|GetTeamComponent _asbp_moba_player_state)))
      (Default|SetDebugText _aswbp_test_text _returnvalue)
      (Development|PrintString (Utilities|String|Append "TeamChange: " "")))))

(event Input|KeyboardEvents|G
  (params (Key :type Key%20Structure :default "None")))

(fn ConstructionScript)