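; Player controller for a MOBA game that handles crosshair enemy targeting, delayed respawn requests and ability cooldown UI.
; Each tick it sphere-traces from screen center out to the attack radius and highlights the crosshair over enemies.
; A newly found enemy becomes the character's AttackTarget through server and multicast events; losing sight does not clear it.
; Respawn goes through the game mode, and cooldown events forward to main UI ability widgets.
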(event Custom|MC_TEST
  (params (Attack%20Target :type Actor%20Object%20Reference))
  (Variables|/Script/MobaDegree.MobaDegreeCharacter|SetAttackTarget (Variables|Default|GetPlayerCharacter) Attack%20Target))

(event Custom|ROS_RequestRespawn
  (Utilities|FlowControl|Delay 3.0)
  (bind _asbp_moba_degree_game_mode (Utilities|Casting|CastToBP_MobaDegreeGameMode (Game|GetGameMode)))
  (Class|GameModeBase|RestartPlayer _asbp_moba_degree_game_mode self))

(event Custom|SERVER_TEST
  (params (Attack%20Target :type Actor%20Object%20Reference))
  (bind _output_get (Variables|/Script/MobaDegree.MobaDegreeCharacter|SetAttackTarget (Variables|Default|GetPlayerCharacter) Attack%20Target))
  (CallFunction|MCTEST _output_get))

(event EventTick
  (params (DeltaSeconds :type Float%20%28single-precision%29))
  (bind _bp_mainui (Variables|Default|GetBP_MainUI))
  (bind _playercharacter (Variables|Default|GetPlayerCharacter))
  (bind (_found _tracedenemy) (CallFunction|StartTraceEnemy))
  (Utilities|IsValid _bp_mainui
    (:Is%20Valid
      (Default|CrosshairEnemyHighlight (Variables|/Game/Blueprints/UI/Widget/MainWidget/UW_MainUI.UW_MainUI_C|GetUW_Crosshair _bp_mainui) _found))
    (:Is%20Not%20Valid
      _))
  (if _found
    (Variables|Default|SetAttackTargetTest _tracedenemy)
    (Utilities|IsValid _playercharacter
      (:Is%20Valid
        (if (not (== (Variables|Default|GetAttackTargetTest) (Variables|/Script/MobaDegree.MobaDegreeCharacter|GetAttackTarget _playercharacter)))
          (CallFunction|SERVERTEST (Variables|Default|GetAttackTargetTest)))))))

(event EventBeginPlay
  (|CallParentFunction))

(event EventInitializeMainWidgetBlueprintVariable
  (bind _asuw_main_ui (Utilities|Casting|CastToUW_MainUI (Variables|Default|GetMainUserWidget)))
  (Variables|Default|SetBP_MainUI _asuw_main_ui))

(event EventGetTraceTarget)

(event EventCallAttackAbilityUICooldown
  (Default|StartAbilityCooldown (Variables|/Game/Blueprints/UI/Widget/MainWidget/UW_MainUI.UW_MainUI_C|GetUW_PlayerAbility_LMB (Variables|Default|GetBP_MainUI))))

(event EventCallRMBAbilityUICooldown
  (Default|StartAbilityCooldown (Variables|/Game/Blueprints/UI/Widget/MainWidget/UW_MainUI.UW_MainUI_C|GetUW_PlayerAbility_RMB (Variables|Default|GetBP_MainUI))))

(event EventCallQAbilityUICooldown
  (Default|StartAbilityCooldown (Variables|/Game/Blueprints/UI/Widget/MainWidget/UW_MainUI.UW_MainUI_C|GetUW_PlayerAbilityQ (Variables|Default|GetBP_MainUI))))

(event EventCallEAbilityUICooldown
  (Default|StartAbilityCooldown (Variables|/Game/Blueprints/UI/Widget/MainWidget/UW_MainUI.UW_MainUI_C|GetUW_PlayerAbilityE (Variables|Default|GetBP_MainUI))))

(event EventCallRAbilityUICooldown
  (Default|StartAbilityCooldown (Variables|/Game/Blueprints/UI/Widget/MainWidget/UW_MainUI.UW_MainUI_C|GetUW_PlayerAbilityUltimate (Variables|Default|GetBP_MainUI))))

(fn ConstructionScript)

(fn PerformTracefromScreen
  (bind (_sizex _sizey) (HUD|GetViewportSize))
  (bind _self self)
  (bind _returnvalue (/ _sizey 2))
  (bind _returnvalue_2 (/ _sizex 2))
  (bind _returnvalue_3 (Math|Conversions|ToFloat(Integer) _returnvalue_2))
  (bind _returnvalue_4 (Math|Conversions|ToFloat(Integer) _returnvalue))
  (bind _returnvalue_5 (Math|Vector2D|MakeVector2D _returnvalue_3 _returnvalue_4))
  (bind (_worldposition _worlddirection) (Class|GameplayStatics|DeprojectScreentoWorld _self _returnvalue_5))
  (bind _outhit (Collision|LineTraceByChannel _worldposition (+ _worldposition (* _worlddirection 2e+03)) "TraceTypeQuery3" false 0 "ForOneFrame"))
  (return _outhit))

(fn StartTraceEnemy
  (bind (_start _end) (CallFunction|GetPlayerScreenTrace (Variables|Default|GetAttackRadius)))
  (bind (_outhit _returnvalue) (Collision|SphereTraceByChannel _start _end 2e+01 "TraceTypeQuery3" false (Utilities|Array|MakeArray (Pawn|GetControlledPawn)) "None" true "(R=1.000000,G=0.000000,B=0.000000,A=1.000000)" "(R=0.000000,G=1.000000,B=0.000000,A=1.000000)" 2.0))
  (if _returnvalue
    (bind _returnvalue_2 (Class|MobaBlueprintFunctionLibrary|IsEnemyActor (Variables|Default|GetPlayerCharacter) (.HitActor (Collision|BreakHitResult _outhit))))
    (if _returnvalue_2
      (return _returnvalue_2 (.HitActor (Collision|BreakHitResult _outhit)))
      (else
        _)))
  (return false 0))

(fn GetAttackTargetfromPlayer
  (return 0))

(fn GetMobaPlayerController
  (return 0))

(fn GetMobaPlayerMesh
  (return 0))

(fn GetPlayerScreenTrace
  (params (Distance :type Float%20%28double-precision%29))
  (bind (_sizex _sizey) (HUD|GetViewportSize))
  (bind _self self)
  (bind _returnvalue (/ _sizey 2))
  (bind _returnvalue_2 (/ _sizex 2))
  (bind _returnvalue_3 (Math|Conversions|ToFloat(Integer) _returnvalue_2))
  (bind _returnvalue_4 (Math|Conversions|ToFloat(Integer) _returnvalue))
  (bind _returnvalue_5 (Math|Vector2D|MakeVector2D _returnvalue_3 _returnvalue_4))
  (bind (_worldposition _worlddirection) (Class|GameplayStatics|DeprojectScreentoWorld _self _returnvalue_5))
  (LocalVariables|SetWorld%20Position _worldposition)
  (LocalVariables|SetWorldDirection (Math|Vector|Normalize _worlddirection))
  (Variables|Default|SetEndTrace (+ (LocalVariables|GetWorld%20Position) (* (LocalVariables|GetWorldDirection) Distance)))
  (return (LocalVariables|GetWorld%20Position) (+ (LocalVariables|GetWorld%20Position) (* (LocalVariables|GetWorldDirection) Distance)) (LocalVariables|GetWorldDirection)))