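; BP_DebugTeamChange is a debug trigger actor that switches a MOBA player's team to its configured TeamToChose.
; On BeginPlay it displays that team on its WBP_TestText widget.
; When a player character overlaps the Box, ServerTeamSet sets the team on the TeamComponent of that player's BP_MobaPlayerState.
; It then calls MCTeamSet, which refreshes the character's debug text through TextDebug.
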(event OnComponentBeginOverlap(Box)
  (params (OverlappedComponent :type Primitive%20Component%20Object%20Reference) (OtherActor :type Actor%20Object%20Reference) (OtherComp :type Primitive%20Component%20Object%20Reference) (OtherBodyIndex :type Integer) (bFromSweep :type Boolean) (SweepResult :type Hit%20Result%20Structure%20%28by%20ref%29))
  (bind _asbp_moba_player_character_base (Utilities|Casting|CastToBP_MobaPlayerCharacterBase OtherActor))
  (bind _asbp_moba_player_state (Utilities|Casting|CastToBP_MobaPlayerState (Variables|/Script/Engine.Pawn|GetPlayerState _asbp_moba_player_character_base)))
  (CallFunction|ServerTeamSet _asbp_moba_player_character_base (Variables|/Script/MobaDegree.MobaPlayerState|GetTeamComponent _asbp_moba_player_state)))

(event Custom|MCTeamSet
  (params (Target :type BP%20Moba%20Player%20Character%20Base%20Object%20Reference))
  (Default|TextDebug Target))

(event Custom|ServerTeamSet
  (params (Target :type BP%20Moba%20Player%20Character%20Base%20Object%20Reference) (Target2 :type Team%20Component%20Object%20Reference))
  (Class|TeamComponent|SetTeam Target2 (Variables|Default|GetTeam%20to%20Chose))
  (CallFunction|MCTeamSet Target))

(event EventBeginPlay
  (bind _aswbp_test_text (Utilities|Casting|CastToWBP_TestText (UserInterface|GetWidget (Variables|Default|GetWidget))))
  (Default|SetDebugText _aswbp_test_text (Variables|Default|GetTeam%20to%20Chose)))

(event Collision|EventActorBeginOverlap
  (params (OtherActor :type Actor%20Object%20Reference)))

(event EventTick
  (params (DeltaSeconds :type Float%20%28single-precision%29)))

(fn ConstructionScript)