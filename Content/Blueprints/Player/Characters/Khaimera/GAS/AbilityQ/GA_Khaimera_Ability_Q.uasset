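; Khaimera's Q gameplay ability, which applies a self-targeted gameplay effect alongside a temporary camera lens effect.
; On a successful commit it starts the Q cooldown UI, adds the lens effect and force-commits the cooldown.
; GE_Khaimera_Ability_Q is applied only with authority.
; After a short fixed delay it clears all camera lens effects and ends, while a failed commit ends it immediately.
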(event Ability|EventActivateAbility
  (bind _returnvalue (Ability|CommitAbility))
  (if _returnvalue
    (bind _bp_mobaplayercontroller (Class|BPIMobaPlayerInterface|GetMobaPlayerController(Message) (Ability|GetAvatarActorfromActorInfo)))
    (Class|MobaDegreePlayerController|CallQAbilityUICooldown _bp_mobaplayercontroller)
    (if _returnvalue
      (bind _asbp_moba_player_character_base (Utilities|Casting|CastToBP_MobaPlayerCharacterBase (Ability|GetAvatarActorfromActorInfo)))
      (Camera|AddGenericCameraLensEffect (Variables|/Script/Engine.PlayerController|GetPlayerCameraManager _bp_mobaplayercontroller) "/Game/Blueprints/Player/Characters/Khaimera/GAS/AbilityQ/BP_Khaimera_Ability_Lens.BP_Khaimera_Ability_Lens_C")
      (Ability|CommitAbilityCooldown false true)
      (if (Ability|HasAuthority (Ability|GetAvatarActorfromActorInfo))
        (GameplayEffects|ApplyGameplayEffectToSelf :self (Ability|GetAbilitySystemComponent _asbp_moba_player_character_base) :GameplayEffectClass "/Game/Blueprints/Player/Characters/Khaimera/GAS/AbilityQ/GE_Khaimera_Ability_Q.GE_Khaimera_Ability_Q_C"))
      (Utilities|FlowControl|Delay 3.0)
      (Class|PlayerCameraManager|ClearCameraLensEffects (Variables|/Script/Engine.PlayerController|GetPlayerCameraManager _bp_mobaplayercontroller))
      (Ability|EndAbility)
      (else
        (Ability|EndAbility)))
    (else
      (Ability|EndAbility))))