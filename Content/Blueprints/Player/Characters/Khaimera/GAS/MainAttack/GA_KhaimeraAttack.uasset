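; Khaimera's main attack gameplay ability, which commits, triggers the attack UI cooldown and forces the ability cooldown as the montage starts.
; It plays a random attack montage section, rerolling to avoid repeating the last one, and waits for the Player.Attack event.
; On that event the server fires a hit cue, applies damage to the player's attack target and adds an attack stack to Khaimera.
; A locally controlled damage-text branch is left unconnected.
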(event Ability|EventActivateAbility
  (bind _returnvalue (Ability|GetAvatarActorfromActorInfo))
  (bind _attacksection (Variables|Default|GetAttackSection))
  (bind _returnvalue_2 (Ability|GetAbilitySystemComponent _returnvalue))
  (bind _returnvalue_3 (Ability|CommitAbility))
  (if _returnvalue_3
    (bind _bp_mobaplayercontroller (Class|BPIMobaPlayerInterface|GetMobaPlayerController(Message) (Ability|GetAvatarActorfromActorInfo)))
    (Class|MobaDegreePlayerController|CallAttackAbilityUICooldown _bp_mobaplayercontroller)
    (if _returnvalue_3
      (bind _asbp_moba_player_character_base (Utilities|Casting|CastToBP_MobaPlayerCharacterBase (Ability|GetAvatarActorfromActorInfo)))
      (Variables|Default|SetRandomIndex (Math|Random|RandomIntegerinRange 0 (- (Utilities|Array|Length _attacksection) 1)) :!label _label)
      (if (== (Variables|Default|GetRandomIndex) (Variables|Default|GetLastAttackIndex))
        (goto _label)
        (else
          (bind _output_get (Variables|Default|SetLastAttackIndex (Variables|Default|GetRandomIndex)))
          (|PlayMontageandWaitforEvent "None" "/Game/Blueprints/Player/Characters/Khaimera/Animations/AM_KhaimeraAttack.AM_KhaimeraAttack" "(GameplayTags=((TagName=\"Player.Attack\")))" 1.0 (Utilities|Array|Get(acopy) _attacksection _output_get) false 1.0
            (:then
              (Ability|CommitAbilityCooldown false true))
            (:OnInterrupted
              (Ability|EndAbility :!label _label_2))
            (:OnCancelled
              (goto _label_2))
            (:EventReceived
              (bind _attacktarget (Class|BPIMobaPlayerInterface|GetAttackTargetfromPlayer(Message) _asbp_moba_player_character_base))
              (Utilities|IsValid _attacktarget
                (:Is%20Valid
                  (Variables|Default|SetAttack%20Target _attacktarget)
                  (Ability|HasAuthority
                    (:True
                      (Class|GameplayAbility|ExecuteGameplayCuewithParams "(TagName=\"GameplayCue.Character.Khaimera.AttackHit\")" (Ability|GameplayCue|MakeGameplayCueParameters :Location (Transformation|GetActorLocation (Variables|Default|GetAttack%20Target))))
                      (GameplayEffects|ApplyGameplayEffectToTarget :self _returnvalue_2 :GameplayEffectClass "/Game/Blueprints/Player/GAS/GE_PlayerDamage.GE_PlayerDamage_C" :Target (Ability|GetAbilitySystemComponent (Variables|Default|GetAttack%20Target)))
                      (GameplayEffects|ApplyGameplayEffectToSelf :self _returnvalue_2 :GameplayEffectClass "/Game/Blueprints/Player/Characters/Khaimera/GAS/MainAttack/GE_KhaimeraS_Attack_Stack.GE_KhaimeraS_Attack_Stack_C")
                      (Ability|EndAbility))
                    (:False
                      (Ability|EndAbility))))
                (:Is%20Not%20Valid
                  (Ability|EndAbility)))))))
      (else
        (Ability|EndAbility)))
    (else
      (Ability|EndAbility))))