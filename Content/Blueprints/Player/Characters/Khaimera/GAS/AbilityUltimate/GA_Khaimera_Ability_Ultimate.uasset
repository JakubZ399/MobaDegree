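; Gameplay Ability for Khaimera's ultimate (R): a montage-driven area attack on nearby enemies.
; Activation notifies cooldown UI, commits, plays the montage and forces the cooldown.
; The montage event triggers a debug-drawn sphere overlap at a mesh socket, applying the RMB ability's GameplayEffect to enemies with a hardcoded damage-text cue.
; The ability ends shortly after the hit, or on failed commit, interruption or cancellation.
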(event Ability|EventActivateAbility
  (bind _radius (Variables|Default|GetRadius))
  (bind _returnvalue (Ability|CommitAbility))
  (bind _bp_mobaplayercontroller (Class|BPIMobaPlayerInterface|GetMobaPlayerController(Message) (Ability|GetAvatarActorfromActorInfo)))
  (Class|MobaDegreePlayerController|CallRAbilityUICooldown _bp_mobaplayercontroller)
  (if _returnvalue
    (bind _asbp_moba_player_character_base (Utilities|Casting|CastToBP_MobaPlayerCharacterBase (Ability|GetAvatarActorfromActorInfo)))
    (|PlayMontageandWaitforEvent "None" "/Game/Blueprints/Player/Characters/Khaimera/Animations/AM_Khaimera_Ability_Ultimate.AM_Khaimera_Ability_Ultimate" "(GameplayTags=((TagName=\"Character.Khaimera.Ability.R\")))" 1.0 "None" false 1.0
      (:then
        (Ability|CommitAbilityCooldown false true))
      (:OnInterrupted
        (Ability|EndAbility :!label _label))
      (:OnCancelled
        (goto _label))
      (:EventReceived
        (Rendering|Debug|DrawDebugSphere (Transformation|GetSocketLocation (Variables|/Script/Engine.Character|GetMesh _asbp_moba_player_character_base) "Ability_Ultimate_Damage") _radius 6 "(R=1.000000,G=1.000000,B=1.000000,A=1.000000)" 4.0)
        (bind _outactors (Collision|SphereOverlapActors (Transformation|GetSocketLocation (Variables|/Script/Engine.Character|GetMesh _asbp_moba_player_character_base) "Ability_Ultimate_Damage") _radius (Utilities|Array|MakeArray "ObjectTypeQuery3" "ObjectTypeQuery7" "ObjectTypeQuery1") 0 (Utilities|Array|MakeArray _asbp_moba_player_character_base)))
        (for _array_element _outactors
          (bind _returnvalue_2 (Class|MobaBlueprintFunctionLibrary|IsEnemyActor _asbp_moba_player_character_base _array_element))
          (if _returnvalue_2
            (GameplayEffects|ApplyGameplayEffectToTarget :self (Ability|GetAbilitySystemComponent _asbp_moba_player_character_base) :GameplayEffectClass "/Game/Blueprints/Player/Characters/Khaimera/GAS/AbilityRMB/GE_Khaimera_Ability_RMB.GE_Khaimera_Ability_RMB_C" :Target (Ability|GetAbilitySystemComponent _array_element))
            (Class|GameplayAbility|ExecuteGameplayCuewithParams "(TagName=\"GameplayCue.Damage.ShowText\")" (Ability|GameplayCue|MakeGameplayCueParameters :RawMagnitude 2.5e+02 :EffectCauser _array_element))))
        (Utilities|FlowControl|Delay 0.2)
        (Ability|EndAbility)))
    (else
      (Ability|EndAbility))))