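; Khaimera's right-click gameplay ability: a leap slam that hits enemies in an area.
; After committing and triggering the UI cooldown, it plays a montage, launches the character forward and up, then spikes gravity for a fast drop.
; A montage event runs a sphere overlap at the leap socket and applies the ability's GameplayEffect to enemies on authority.
; The ability then ends, lowering gravity again only if the overlap found actors.
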(event Ability|EventActivateAbility
  (bind _radius (Variables|Default|GetRadius))
  (bind _returnvalue (Ability|CommitAbility))
  (if _returnvalue
    (bind _bp_mobaplayercontroller (Class|BPIMobaPlayerInterface|GetMobaPlayerController(Message) (Ability|GetAvatarActorfromActorInfo)))
    (Class|MobaDegreePlayerController|CallRMBAbilityUICooldown _bp_mobaplayercontroller)
    (if _returnvalue
      (bind _asbp_moba_player_character_base (Utilities|Casting|CastToBP_MobaPlayerCharacterBase (Ability|GetAvatarActorfromActorInfo)))
      (Variables|/Script/Engine.CharacterMovementComponent|SetGravityScale (Variables|/Script/Engine.Character|GetCharacterMovement _asbp_moba_player_character_base) 1.5)
      (|PlayMontageandWaitforEvent "None" "/Game/Blueprints/Player/Characters/Khaimera/Animations/AM_Khaimera_Ability_RMB.AM_Khaimera_Ability_RMB" "(GameplayTags=((TagName=\"Character.Khaimera.Ability.RMB\")))" 1.0 "None" false 1.0
        (:then
          (Character|LaunchCharacter _asbp_moba_player_character_base (+ (* (Math|Vector|Normalize (Transformation|GetActorForwardVector (Ability|GetAvatarActorfromActorInfo))) 1.2e+03) "0.000000,0.000000,2200.000000") true true)
          (Utilities|FlowControl|Delay 0.2)
          (Variables|/Script/Engine.CharacterMovementComponent|SetGravityScale (Variables|/Script/Engine.Character|GetCharacterMovement _asbp_moba_player_character_base) 17.0))
        (:OnCompleted
          (Ability|EndAbility :!label _label))
        (:OnInterrupted
          (goto _label))
        (:OnCancelled
          (goto _label))
        (:EventReceived
          (if (Variables|Default|GetbDebugAbility)
            (Rendering|Debug|DrawDebugSphere (Transformation|GetSocketLocation (Variables|/Script/Engine.Character|GetMesh _asbp_moba_player_character_base) "FX_Leap_AOE") _radius 12 "(R=1.000000,G=0.000000,B=0.246613,A=1.000000)" 3.0))
          (bind (_outactors _returnvalue_2) (Collision|SphereOverlapActors (Transformation|GetSocketLocation (Variables|/Script/Engine.Character|GetMesh _asbp_moba_player_character_base) "FX_Leap_AOE") _radius (Utilities|Array|MakeArray "ObjectTypeQuery3" "ObjectTypeQuery7" "ObjectTypeQuery1") 0 (Utilities|Array|MakeArray _asbp_moba_player_character_base)))
          (if _returnvalue_2
            (for _array_element _outactors
              (bind _returnvalue_3 (Class|MobaBlueprintFunctionLibrary|IsEnemyActor _asbp_moba_player_character_base _array_element))
              (if _returnvalue_3
                (Ability|HasAuthority
                  (:True
                    (GameplayEffects|ApplyGameplayEffectToTarget :self (Ability|GetAbilitySystemComponent _asbp_moba_player_character_base) :GameplayEffectClass "/Game/Blueprints/Player/Characters/Khaimera/GAS/AbilityRMB/GE_Khaimera_Ability_RMB.GE_Khaimera_Ability_RMB_C" :Target (Ability|GetAbilitySystemComponent _array_element))))))
            (Utilities|FlowControl|Delay 0.2)
            (Ability|EndAbility)
            (Variables|/Script/Engine.CharacterMovementComponent|SetGravityScale (Variables|/Script/Engine.Character|GetCharacterMovement _asbp_moba_player_character_base) 1.5)
            (else
              (Ability|EndAbility)))))
      (else
        (Ability|EndAbility)))
    (else
      (Ability|EndAbility))))