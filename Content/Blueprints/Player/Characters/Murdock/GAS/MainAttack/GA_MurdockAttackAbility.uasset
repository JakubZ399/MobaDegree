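; Gameplay ability for Murdock's main attack, built on the Gameplay Ability System.
; It commits, plays the attack montage and forces the cooldown as playback begins.
; On the montage's attack event, the server applies damage to the character's AttackTarget and fires the attack gameplay cue.
; That event, interruption or cancellation ends the ability without stopping the montage, and OnEndAbility prints a debug string.
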(event Ability|EventActivateAbility
  (bind _returnvalue (Ability|CommitAbility))
  (if _returnvalue
    (bind _asbp_moba_player_character_base (Utilities|Casting|CastToBP_MobaPlayerCharacterBase (Ability|GetAvatarActorfromActorInfo)))
    (|PlayMontageandWaitforEvent "None" "/Game/Blueprints/Player/Characters/Murdock/Animations/AM_MurdockAttack.AM_MurdockAttack" "(GameplayTags=((TagName=\"Player.Attack\")))" 1.0 "Attack1" false 1.0
      (:then
        (Ability|CommitAbilityCooldown false true))
      (:OnInterrupted
        (Ability|EndAbility :!label _label))
      (:OnCancelled
        (goto _label))
      (:EventReceived
        (if (Ability|HasAuthority (Ability|GetAvatarActorfromActorInfo))
          (GameplayEffects|ApplyGameplayEffectToTarget :self (Ability|GetAbilitySystemComponent _asbp_moba_player_character_base) :GameplayEffectClass "/Game/Blueprints/Player/Characters/Murdock/GAS/MainAttack/GE_MurdockAttackDamage.GE_MurdockAttackDamage_C" :Target (Ability|GetAbilitySystemComponent (Variables|/Script/MobaDegree.MobaDegreeCharacter|GetAttackTarget _asbp_moba_player_character_base)) :Level 1.0)
          (Class|GameplayAbility|ExecuteGameplayCuewithParams "(TagName=\"GameplayCue.Character.Murdock.Attack\")" (Ability|GameplayCue|MakeGameplayCueParameters :EffectCauser _asbp_moba_player_character_base))
          (Ability|EndAbility)
          (else
            (Ability|EndAbility)))))
    (else
      (Ability|EndAbility))))

(event Ability|EventOnEndAbility
  (params (bWasCancelled :type Boolean))
  (Development|PrintString "Hello"))