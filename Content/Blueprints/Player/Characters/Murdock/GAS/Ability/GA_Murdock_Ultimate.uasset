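; Murdock's ultimate gameplay ability, apparently an unfinished beam attack.
; On activation it commits, checks for a player-controlled MOBA character, then runs a debug-drawn multi sphere trace whose end scales location plus forward vector together.
; Trace hits are unused and the ability only ends when commit fails.
; Disconnected leftover logic holds server-side GE_MurdockAttackDamage application to AttackTarget, a muzzle beam emitter and attack-state reset.
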(event Ability|EventActivateAbility
  (bind _returnvalue (Ability|GetAvatarActorfromActorInfo))
  (bind _returnvalue_2 (Transformation|GetActorLocation _returnvalue))
  (bind _returnvalue_3 (Ability|CommitAbility))
  (if _returnvalue_3
    (bind _asbp_moba_player_character_base (Utilities|Casting|CastToBP_MobaPlayerCharacterBase _returnvalue))
    (Utilities|Casting|CastToPlayerController (Pawn|GetController _asbp_moba_player_character_base))
    (Collision|MultiSphereTraceByChannel _returnvalue_2 (* (+ _returnvalue_2 (Transformation|GetActorForwardVector _returnvalue)) 1e+01) 2e+01 "TraceTypeQuery1" false 0 "Persistent")
    (else
      (Ability|EndAbility))))