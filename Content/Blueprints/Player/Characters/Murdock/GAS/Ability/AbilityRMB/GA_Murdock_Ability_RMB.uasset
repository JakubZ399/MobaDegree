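; Murdock's right-click gameplay ability, a spreadshot that damages and knocks back nearby enemies.
; On commit it starts the UI cooldown, plays a montage, forces the ability cooldown and waits for a gameplay event.
; That event triggers a sphere overlap at the SpreadshotHit socket.
; On the server, enemies receive a damage effect, and characters are launched away from Murdock with slight lift and a hit GameplayCue.
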(event Ability|EventActivateAbility
  (bind _returnvalue (Ability|GetAvatarActorfromActorInfo))
  (bind _returnvalue_2 (Ability|GetAvatarActorfromActorInfo))
  (bind _returnvalue_3 (Ability|CommitAbility))
  (if _returnvalue_3
    (bind _bp_mobaplayercontroller (Class|BPIMobaPlayerInterface|GetMobaPlayerController(Message) _returnvalue_2))
    (Class|MobaDegreePlayerController|CallRMBAbilityUICooldown _bp_mobaplayercontroller)
    (bind _ascharacter (Utilities|Casting|CastToCharacter _returnvalue_2)
      (:then
        (|PlayMontageandWaitforEvent "None" "/Game/Blueprints/Player/Characters/Murdock/Animations/AM_Murdock_Ability_RMB.AM_Murdock_Ability_RMB" "(GameplayTags=((TagName=\"Character.Murdock.Ability.RMB\")))" 1.0 "Default" true 1.0
          (:then
            (Ability|CommitAbilityCooldown false true))
          (:EventReceived
            (bind (_outactors _returnvalue_4) (Collision|SphereOverlapActors (Transformation|GetSocketLocation (Variables|/Script/Engine.Character|GetMesh _ascharacter) "SpreadshotHit") (Variables|Default|GetRadius) (Utilities|Array|MakeArray "ObjectTypeQuery3" "ObjectTypeQuery7" "ObjectTypeQuery1") 0 (Utilities|Array|MakeArray _ascharacter)))
            (if _returnvalue_4
              (for _array_element _outactors
                (bind _output_get (Variables|Default|SetHitActor _array_element))
                (bind _returnvalue_5 (Class|MobaBlueprintFunctionLibrary|IsEnemyActor _returnvalue _output_get))
                (if _returnvalue_5
                  (Ability|HasAuthority
                    (:True
                      (GameplayEffects|ApplyGameplayEffectToTarget :self (Ability|GetAbilitySystemComponent _returnvalue) :GameplayEffectClass "/Game/Blueprints/Player/Characters/Murdock/GAS/Ability/AbilityRMB/GE_Murdock_Ability_RMB_Damage.GE_Murdock_Ability_RMB_Damage_C" :Target (Ability|GetAbilitySystemComponent (Variables|Default|GetHitActor)))
                      (bind _output_get_2 (Variables|Default|SetDirection (Math|Vector|MakeVector (.x (- (Transformation|GetActorLocation (Variables|Default|GetHitActor)) (Transformation|GetActorLocation (Ability|GetAvatarActorfromActorInfo)))) (.y (- (Transformation|GetActorLocation (Variables|Default|GetHitActor)) (Transformation|GetActorLocation (Ability|GetAvatarActorfromActorInfo)))) 0.0)))
                      (Variables|Default|SetDirection (Math|Vector|Normalize _output_get_2))
                      (Variables|Default|SetVelocity (+ (* (Variables|Default|GetDirection) (Variables|Default|GetStrenght)) "0.000000,0.000000,50.000000"))
                      (bind _ascharacter_2 (Utilities|Casting|CastToCharacter (Variables|Default|GetHitActor)))
                      (Character|LaunchCharacter _ascharacter_2 (Variables|Default|GetVelocity) true true)
                      (Class|GameplayAbility|ExecuteGameplayCuewithParams "(TagName=\"GameplayCue.Character.Murdock.Ability.RMB.Hit\")" (Ability|GameplayCue|MakeGameplayCueParameters :RawMagnitude 2.5e+02 :Location (Transformation|GetActorLocation (Variables|Default|GetHitActor))))))))
              (Ability|EndAbility)
              (else
                (Ability|EndAbility))))))
      (:CastFailed
        (Ability|EndAbility)))))