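; Gameplay ability for Murdock's Q, which fires a Tazer Tap projectile.
; After committing, it triggers the Q cooldown UI through the MOBA player controller message interface and plays the Q montage.
; A montage gameplay event spawns the projectile at the TazerTapSpawn socket with the character's rotation, passing the character as owning player.
; The ability ends shortly after spawning, or on failed commit, failed Character cast, interruption or cancellation.
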(event Ability|EventActivateAbility
  (bind _returnvalue (Ability|GetAvatarActorfromActorInfo))
  (bind _returnvalue_2 (Ability|CommitAbility))
  (if _returnvalue_2
    (bind _bp_mobaplayercontroller (Class|BPIMobaPlayerInterface|GetMobaPlayerController(Message) _returnvalue))
    (Class|MobaDegreePlayerController|CallQAbilityUICooldown _bp_mobaplayercontroller)
    (bind _ascharacter (Utilities|Casting|CastToCharacter _returnvalue)
      (:then
        (Variables|Default|SetCharacter _ascharacter)
        (|PlayMontageandWaitforEvent "None" "/Game/Blueprints/Player/Characters/Murdock/Animations/AM_Murdock_Ability_Q.AM_Murdock_Ability_Q" "(GameplayTags=((TagName=\"Character.Murdock.Ability.Q\")))" 1.0 "None" true 1.0
          (:OnInterrupted
            _)
          (:OnCancelled
            _)
          (:EventReceived
            (Game|SpawnActorfromClass "/Game/Blueprints/Player/Characters/Murdock/GAS/Ability/AbilityQ/BP_Murdock_TazerTap_Projectile.BP_Murdock_TazerTap_Projectile_C" (Math|Transform|MakeTransform (Transformation|GetSocketLocation (Variables|/Script/Engine.Character|GetMesh (Variables|Default|GetCharacter)) "TazerTapSpawn") (Transformation|GetActorRotation (Variables|Default|GetCharacter))) "Undefined" "MultiplyWithRoot" 0 (Variables|Default|GetCharacter) 0)
            (Utilities|FlowControl|Delay 0.3)))
        (Ability|EndAbility))
      (:CastFailed
        (Ability|EndAbility)))
    (else
      (Ability|EndAbility))))

(event Ability|EventOnEndAbility
  (params (bWasCancelled :type Boolean)))