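; Murdock's Q ability in GAS: a laser attack that damages enemies in a line toward his current attack target.
; It commits, plays the attack montage and, on the event tag, fires a laser cue and sphere-traces pawns along that line, with debug drawing on.
; Opposing-team hits, except minion groups, get a hit cue and an authority-only damage effect, then combat state returns to Idle.
; A decal preview chain is left unconnected.
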(event Ability|EventActivateAbility
  (bind _returnvalue (Ability|CommitAbility))
  (if _returnvalue
    (bind _asbp_moba_player_character_base (Utilities|Casting|CastToBP_MobaPlayerCharacterBase (Ability|GetAvatarActorfromActorInfo)))
    (Variables|Default|SetMoba%20Player%20Character%20Base _asbp_moba_player_character_base)
    (|PlayMontageandWaitforEvent "None" "/Game/Blueprints/Player/Characters/Murdock/Animations/AM_Murdock_AbilityQ.AM_Murdock_AbilityQ" "(GameplayTags=((TagName=\"Player.Attack\")))" 0.9 "Attack1" false 1.0
      (:then
        (Ability|CommitAbilityCooldown false true))
      (:OnBlendOut
        (Ability|EndAbility :!label _label))
      (:OnInterrupted
        (goto _label))
      (:OnCancelled
        (goto _label))
      (:EventReceived
        (Class|GameplayAbility|ExecuteGameplayCuewithParams "(TagName=\"GameplayCue.Character.Murdock.Ability.Q.Laser\")" (Ability|GameplayCue|MakeGameplayCueParameters :EffectCauser (Variables|Default|GetMoba%20Player%20Character%20Base)))
        (bind _outhits (Collision|MultiSphereTraceForObjects (Math|Vector|MakeVector (.x (+ (Transformation|GetActorLocation (Variables|Default|GetMoba%20Player%20Character%20Base)) (* (Math|Vector|Normalize (- (Transformation|GetActorLocation (Variables|/Script/MobaDegree.MobaDegreeCharacter|GetAttackTarget (Variables|Default|GetMoba%20Player%20Character%20Base))) (Transformation|GetActorLocation (Variables|Default|GetMoba%20Player%20Character%20Base)))) 1e+02))) (.y (+ (Transformation|GetActorLocation (Variables|Default|GetMoba%20Player%20Character%20Base)) (* (Math|Vector|Normalize (- (Transformation|GetActorLocation (Variables|/Script/MobaDegree.MobaDegreeCharacter|GetAttackTarget (Variables|Default|GetMoba%20Player%20Character%20Base))) (Transformation|GetActorLocation (Variables|Default|GetMoba%20Player%20Character%20Base)))) 1e+02))) (- (.Z (Math|Vector|BreakVector (Transformation|GetActorLocation (Variables|Default|GetMoba%20Player%20Character%20Base)))) 8e+01)) (Math|Vector|MakeVector (.x (+ (Transformation|GetActorLocation (Variables|Default|GetMoba%20Player%20Character%20Base)) (* (Math|Vector|Normalize (- (Transformation|GetActorLocation (Variables|/Script/MobaDegree.MobaDegreeCharacter|GetAttackTarget (Variables|Default|GetMoba%20Player%20Character%20Base))) (Transformation|GetActorLocation (Variables|Default|GetMoba%20Player%20Character%20Base)))) 8e+02))) (.y (+ (Transformation|GetActorLocation (Variables|Default|GetMoba%20Player%20Character%20Base)) (* (Math|Vector|Normalize (- (Transformation|GetActorLocation (Variables|/Script/MobaDegree.MobaDegreeCharacter|GetAttackTarget (Variables|Default|GetMoba%20Player%20Character%20Base))) (Transformation|GetActorLocation (Variables|Default|GetMoba%20Player%20Character%20Base)))) 8e+02))) (- (.Z (Math|Vector|BreakVector (Transformation|GetActorLocation (Variables|Default|GetMoba%20Player%20Character%20Base)))) 8e+01)) 85.0 (Utilities|Array|MakeArray "ObjectTypeQuery3") false 0 "ForDuration"))
        (if (Utilities|Array|IsNotEmpty _outhits)
          (bind _returnvalue_2 (Class|MobaTeamInterface|GetTeamInterface(Message) (Variables|Default|GetMoba%20Player%20Character%20Base)))
          (Variables|Default|SetPlayerTeam _returnvalue_2)
          (for _array_element _outhits
            (if (Utilities|DoesObjectImplementInterface (.HitActor (Collision|BreakHitResult _array_element)) "/Script/MobaDegree.MobaTeamInterface")
              (bind _returnvalue_3 (Class|MobaTeamInterface|GetTeamInterface(Message) (.HitActor (Collision|BreakHitResult _array_element))))
              (if (Utilities|Enum|NotEqual(Enum) _returnvalue_3 (Variables|Default|GetPlayerTeam))
                (if (!= (.HitActor (Collision|BreakHitResult _array_element)) "/Game/Blueprints/Minions/BP_MinionGroup.BP_MinionGroup")
                  (Class|GameplayAbility|ExecuteGameplayCuewithParams "(TagName=\"GameplayCue.Character.Murdock.Ability.Q.Hit\")" (Ability|GameplayCue|MakeGameplayCueParameters :Location (Transformation|GetActorLocation (.HitActor (Collision|BreakHitResult _array_element)))))
                  (if (Ability|HasAuthority (Ability|GetAvatarActorfromActorInfo))
                    (GameplayEffects|ApplyGameplayEffectToTarget :self (Ability|GetAbilitySystemComponent (Variables|Default|GetMoba%20Player%20Character%20Base)) :GameplayEffectClass "/Game/Blueprints/Player/Characters/Murdock/GAS/Ability/AbilityQ/GE_MurdockAbilityQDamage.GE_MurdockAbilityQDamage_C" :Target (Ability|GetAbilitySystemComponent (.HitActor (Collision|BreakHitResult _array_element))) :Level 1.0))))))
          (Class|MobaDegreeCharacter|SetCombatState (Variables|Default|GetMoba%20Player%20Character%20Base) "Idle")
          (Ability|EndAbility)
          (else
            (Class|MobaDegreeCharacter|SetCombatState (Variables|Default|GetMoba%20Player%20Character%20Base) "Idle")
            (Ability|EndAbility)))))
    (else
      (Ability|EndAbility))))