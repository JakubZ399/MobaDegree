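; Gameplay ability for a minion's ranged attack, firing a projectile at the target supplied by the avatar's EnemyInfoAIMessage.
; It plays the attack montage and waits for a Tower.Shoot gameplay event, reusing BP_TowerShot as a scaled, short-lived projectile spawned at the muzzle socket.
; On montage completion or interruption, it signals attack end through an interface call and ends the ability.
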(event Ability|EventActivateAbility
  (bind (_meshcomponent _attacktargetref _selfref) (Class|MinionAI|EnemyInfoAI(Message) (Ability|GetAvatarActorfromActorInfo)))
  (Animation|Montage|PlayMontage _meshcomponent "/Game/Blueprints/Minions/Animations/AM_AttackMinionRange.AM_AttackMinionRange"
    (:then
      (Ability|Tasks|WaitGameplayEvent "(TagName=\"Tower.Shoot\")" 0
        (:EventReceived
          (bind _returnvalue (Game|SpawnActorfromClass "/Game/Blueprints/Actor/Tower/TowerShot/BP_TowerShot.BP_TowerShot_C" (Math|Transform|MakeTransform (.location (Transformation|GetSocketTransform _meshcomponent "Muzzle_Front" "RTS_World")) (.rotation (Transformation|GetSocketTransform _meshcomponent "Muzzle_Front" "RTS_World")) "0.400000,0.400000,0.400000") "Undefined" "MultiplyWithRoot" 0 0))
          (Class|TowerShot|AttackTarget _returnvalue _attacktargetref)
          (Actor|SetLifeSpan _returnvalue 1.5))))
    (:OnCompleted
      (Class|MinionBase|CallonAttackEndInterfaceImplementation _selfref :!label _label)
      (Ability|EndAbility))
    (:OnInterrupted
      (goto _label))))

(event Ability|EventOnEndAbility
  (params (bWasCancelled :type Boolean)))