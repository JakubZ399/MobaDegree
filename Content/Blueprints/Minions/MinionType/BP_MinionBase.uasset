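; Base minion character for team-based groups, with a Blue or Red mesh, an outline toggle and attacks run through the Gameplay Ability System.
; Attributes supply walk speed and attack radius, and BeginPlay grants the BaseAttack ability.
; The minion group's target event and the HomeBase location feed the AI blackboard.
; While HomeBase is valid, Tick also polls an attribute and at zero unpossesses, broadcasts death, spawns VFX and expires the actor.
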(event Custom|SetupAttackTarget
  (params (AttackTarget :type Actor%20Object%20Reference))
  ;[1 0 0] Comment
  (bind _output_get (Variables|Default|SetAttackTarget AttackTarget))
  (AI|Components|Blackboard|SetValueasObject (AI|GetBlackboard (AI|GetAIController self)) (Utilities|Name|MakeLiteralName "AttackTarget") _output_get))

(event Custom|BindOnAttackTarget
  (params (MinionGroup :type BP%20Minion%20Group%20Object%20Reference))
  ;[1 0 0] Comment
  (EventDispatchers|BindEventtoOnAttackTargetSet MinionGroup (delegate Custom|SetupAttackTarget)))

(event Custom|SetGroupPosition
  (params (GroupPosition :type Vector))
  (bind _self self)
  (bind _returnvalue (AI|GetAIController _self))
  ;[1 0 0] Comment
  (bind _output_get (Variables|Default|SetGroupPosition GroupPosition))
  (Utilities|IsValid _returnvalue
    (:Is%20Valid
      (AI|Components|Blackboard|SetValueasVector (AI|GetBlackboard _returnvalue) (Variables|Default|GetGroupPositionKey) _output_get))))

(event Custom|Attack
  ;[1 0 0] Comment
  (Abilities|TryActivateAbilitybyClass (Variables|Default|GetAbilitySystemComponent) (Variables|Default|GetBaseAttack) true)
  (bind _attacktarget (CallFunction|GetAttackTarget))
  (Rendering|Debug|DrawDebugSphere (Transformation|GetActorLocation _attacktarget) 5e+01 12 "(R=1.000000,G=0.213542,B=0.686260,A=1.000000)" 1.0 3.0))

(event Custom|ChangeMesh
  ;[1 0 0] Added
  (bind _returnvalue (Class|TeamComponent|GetTeam (Variables|Default|GetTeamComponent)))
  (switch Utilities|FlowControl|Switch|SwitchonEGameTeam _returnvalue
    (:Blue
      (bind _blueminionmesh (Variables|Default|GetBlueMinionMesh)
        (:then
          (Variables|/Script/Engine.SkeletalMeshComponent|SetSkeletalMeshAsset (Variables|Character|GetMesh) _blueminionmesh))
        (:else)))
    (:Red
      (bind _redminionmesh (Variables|Default|GetRedMinionMesh)
        (:then
          (Variables|/Script/Engine.SkeletalMeshComponent|SetSkeletalMeshAsset (Variables|Character|GetMesh) _redminionmesh))
        (:else)))))

(event EventBeginPlay
  ;[1 0 0 0.5] Comment
  (Variables|/Script/Engine.CharacterMovementComponent|SetMaxWalkSpeed (Variables|Character|GetCharacterMovement) (.ReturnValue (Class|AbilitySystemComponent|GetGameplayAttributeValue (Variables|Default|GetAbilitySystemComponent) "(AttributeName=\"MovementSpeed\",Attribute=/Script/MobaDegree.MobaAttributeSet:MovementSpeed,AttributeOwner=\"/Script/CoreUObject.Class'/Script/MobaDegree.MobaAttributeSet'\")")))
  (GameplayAbilities|GiveAbility (Variables|Default|GetAbilitySystemComponent) (Variables|Default|GetBaseAttack) 0 -1))

(event EventShowOutline
  (params (EnableOutline :type Boolean))
  ;[1 0 0] Comment
  (Rendering|SetRenderCustomDepth (Variables|Character|GetMesh) EnableOutline))

(event EventCallonAttackEndInterface
  ;[1 0 0] Comment
  (Default|CallOnAttackEnd))

(event EventTick
  (params (DeltaSeconds :type Float%20%28single-precision%29))
  (bind _self self)
  (bind _returnvalue (AI|GetAIController _self))
  ;[1 0 0] Comment
  (bind _homebase (Variables|Default|GetHomeBase)
    (:then
      (CallFunction|SetGroupPosition (Transformation|GetWorldLocation _homebase))
      (if (<= (.ReturnValue (Class|AbilitySystemComponent|GetGameplayAttributeValue (Variables|Default|GetAbilitySystemComponent) "(AttributeName=\"Health\",Attribute=/Script/MobaDegree.MobaAttributeSet:Health,AttributeOwner=\"/Script/CoreUObject.Class'/Script/MobaDegree.MobaAttributeSet'\")")) 0.0)
        (Utilities|FlowControl|DoOnce false
          (:Completed
            (Variables|/Script/AIModule.AIController|SetbStopAILogicOnUnposses _returnvalue false)
            (Pawn|UnPossess _returnvalue)
            (Default|CallOnMinionDeath)
            (Actor|SetLifeSpan 0.2)
            (Effects|SpawnEmitteratLocation (Variables|Default|GetDeathVFX) (Transformation|GetActorLocation))))))
    (:else)))

(fn ConstructionScript)

(fn GetAttackTarget
  (return (Variables|Default|GetAttackTarget)))

(fn GetAttackRadius
  (return (.ReturnValue (Class|AbilitySystemComponent|GetGameplayAttributeValue (Variables|Default|GetAbilitySystemComponent) "(AttributeName=\"AttackRange\",Attribute=/Script/MobaDegree.MobaAttributeSet:AttackRange,AttributeOwner=\"/Script/CoreUObject.Class'/Script/MobaDegree.MobaAttributeSet'\")"))))

(fn GetTeamInterface
  (bind _returnvalue (Class|TeamComponent|GetTeamInterfaceImplementation (Variables|Default|GetTeamComponent)))
  (return _returnvalue))

(fn EnemyInfoAI
  (return (Variables|Character|GetMesh) (Variables|Default|GetAttackTarget) self))

(fn GetAttackRadiusAttribute
  (bind _attackradius (CallFunction|GetAttackRadius))
  (return _attackradius))

(fn GetMinionRef
  (return self))