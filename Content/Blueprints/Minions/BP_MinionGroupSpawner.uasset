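; BP_MinionGroupSpawner is an actor that periodically spawns groups of minions for a team along a lane.
; On BeginPlay it spawns a group at once, then repeats on a looping timer set by TimeToSpawnGroup.
; Each BP_MinionGroup appears at the spawner's root transform, receives the spawner's Team and EnemyLaneTarget, and is then initialized.
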(event Custom|SpawnMinionGroup
  (bind _returnvalue (Game|SpawnActorfromClass "/Game/Blueprints/Minions/BP_MinionGroup.BP_MinionGroup_C" (Transformation|GetWorldTransform (Variables|Default|GetDefaultSceneRoot)) "Undefined" "MultiplyWithRoot" 0 0))
  (Variables|/Game/Blueprints/Minions/BP_MinionGroup.BP_MinionGroup_C|SetTeam _returnvalue (Variables|ToSetup|GetTeam))
  (Variables|/Game/Blueprints/Minions/BP_MinionGroup.BP_MinionGroup_C|SetEnemyLaneTarget _returnvalue (Variables|ToSetup|GetEnemy%20Lane%20Target))
  (Default|Initialize _returnvalue))

(event EventBeginPlay
  (CallFunction|SpawnMinionGroup)
  (Utilities|Time|SetTimerbyEvent (delegate Custom|SpawnMinionGroup) (Variables|Default|GetTimeToSpawnGroup) true))

(fn ConstructionScript)