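; BP_MinionBase is a base minion Blueprint that takes an attack target and moves toward it.
; SetupAttackTarget stores the target, issues an AI MoveTo to its location at that moment, and sets the hasSeenPlayer Blackboard flag without waiting for arrival.
; GetAttackTarget exposes the stored target, while the PawnSensing OnSeePawn event is present but empty.
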(event OnSeePawn(PawnSensing)
  (params (Pawn :type Pawn%20Object%20Reference)))

(event Custom|SetupAttackTarget
  (params (AttackTargetr :type Actor%20Object%20Reference))
  (bind _output_get (Variables|Default|SetAttackTarget AttackTargetr))
  (AI|AIMoveTo self (Transformation|GetActorLocation _output_get) 0 3e+01 false
    (:then
      (AI|Components|Blackboard|SetValueasBool (AI|GetBlackboard (AI|GetAIController self)) (Utilities|Name|MakeLiteralName "hasSeenPlayer") true))))

(event EventBeginPlay)

(event Collision|EventActorBeginOverlap
  (params (OtherActor :type Actor%20Object%20Reference)))

(event EventTick
  (params (DeltaSeconds :type Float%20%28single-precision%29)))

(fn ConstructionScript)

(fn GetAttackTarget
  (return (Variables|Default|GetAttackTarget)))