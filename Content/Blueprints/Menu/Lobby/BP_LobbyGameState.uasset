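; Lobby game state that manages Blue and Red team rosters for a MOBA match.
; UpdatePlayersUI adds joining players to the smaller team, favoring Blue on ties, and ChangeTeam swaps a player between the arrays by name.
; Both rosters replicate with RepNotify, firing OnPlayerListChange on updates.
; StartGame matches PlayerArray names against the rosters to set the team on each BP_MobaPlayerState's TeamComponent; an older EventGraph copy is disconnected.
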(event Custom|UpdatePlayersUI
  (params (LobbyPlayerController :type BP%20Lobby%20Player%20Controller%20Object%20Reference))
  (bind _redteamplayerinfo (Variables|Default|GetRedTeamPlayerInfo))
  (bind _blueteamplayerinfo (Variables|Default|GetBlueTeamPlayerInfo))
  (bind _playerstate (Variables|/Script/Engine.Controller|GetPlayerState LobbyPlayerController))
  (bind _returnvalue (Utilities|Array|Length _blueteamplayerinfo))
  (bind _returnvalue_2 (Utilities|Array|Length _redteamplayerinfo))
  (bind _returnvalue_3 (PlayerState|GetPlayerName _playerstate))
  (bind _playerid (Variables|/Script/Engine.PlayerState|GetPlayerId _playerstate))
  (bind _returnvalue_4 (Utilities|String|ToString(Integer) _playerid))
  (if (<= _returnvalue _returnvalue_2)
    (Utilities|Array|AddUnique (Variables|Default|GetBlueTeamPlayerInfo) (Utilities|Struct|MakePlayerInfoLobby _returnvalue_4 _returnvalue_3 "Blue" false))
    (Default|CallOnPlayerListChange :!label _label)
    (elif (> _returnvalue _returnvalue_2)
      (Utilities|Array|AddUnique (Variables|Default|GetRedTeamPlayerInfo) (Utilities|Struct|MakePlayerInfoLobby _returnvalue_4 _returnvalue_3 "Red" false))
      (goto _label))))

(fn ConstructionScript)

(fn OnRepRedTeamPlayerInfo
  (Default|CallOnPlayerListChange))

(fn OnRepBlueTeamPlayerInfo
  (Default|CallOnPlayerListChange))

(fn ChangeTeam
  (params (PlayerState :type Player%20State%20Object%20Reference))
  (LocalVariables|SetLobbyPlayerState PlayerState)
  (for (_array_element _array_index) (Variables|Default|GetBlueTeamPlayerInfo)
    (if (Utilities|Enum|Equal(Enum) (.PlayerName (Utilities|Struct|BreakPlayerInfoLobby _array_element)) (PlayerState|GetPlayerName (LocalVariables|GetLobbyPlayerState)))
      (Utilities|Array|RemoveIndex (Variables|Default|GetBlueTeamPlayerInfo) _array_index)
      (Utilities|Array|AddUnique (Variables|Default|GetRedTeamPlayerInfo) (Utilities|Struct|MakePlayerInfoLobby (Utilities|String|ToString(Integer) (Variables|/Script/Engine.PlayerState|GetPlayerId (LocalVariables|GetLobbyPlayerState))) (PlayerState|GetPlayerName (LocalVariables|GetLobbyPlayerState)) "Red" false))
      (Networking|SwitchHasAuthority
        (:Authority
          (Default|CallOnPlayerListChange)
          (return))
        (:Remote
          (return)))))
  (for (_array_element_2 _array_index_2) (Variables|Default|GetRedTeamPlayerInfo)
    (if (Utilities|Enum|Equal(Enum) (.PlayerName (Utilities|Struct|BreakPlayerInfoLobby _array_element_2)) (PlayerState|GetPlayerName (LocalVariables|GetLobbyPlayerState)))
      (Utilities|Array|RemoveIndex (Variables|Default|GetRedTeamPlayerInfo) _array_index_2)
      (Utilities|Array|AddUnique (Variables|Default|GetBlueTeamPlayerInfo) (Utilities|Struct|MakePlayerInfoLobby (Utilities|String|ToString(Integer) (Variables|/Script/Engine.PlayerState|GetPlayerId (LocalVariables|GetLobbyPlayerState))) (PlayerState|GetPlayerName (LocalVariables|GetLobbyPlayerState)) "Blue" false))
      (Networking|SwitchHasAuthority
        (:Authority
          (Default|CallOnPlayerListChange)
          (return))
        (:Remote
          (return)))))
  (return))

(fn StartGame
  (for _array_element (Variables|Default|GetPlayerArray)
    (bind _asbp_moba_player_state (Utilities|Casting|CastToBP_MobaPlayerState _array_element))
    (bind _array_element_2 (Utilities|Array|ForEachLoopwithBreak (Variables|Default|GetRedTeamPlayerInfo))
      (:LoopBody
        (if (Utilities|Enum|Equal(Enum) (.PlayerName (Utilities|Struct|BreakPlayerInfoLobby _array_element_2)) (PlayerState|GetPlayerName _asbp_moba_player_state))
          (Class|TeamComponent|SetTeam (Variables|/Script/MobaDegree.MobaPlayerState|GetTeamComponent _asbp_moba_player_state) "Red")
          (Development|PrintString "RED" true true "(R=1.000000,G=0.000000,B=0.053420,A=1.000000)")
          (return)))
      (:Completed
        (bind _array_element_3 (Utilities|Array|ForEachLoopwithBreak (Variables|Default|GetBlueTeamPlayerInfo))
          (:LoopBody
            (if (Utilities|Enum|Equal(Enum) (.PlayerName (Utilities|Struct|BreakPlayerInfoLobby _array_element_3)) (PlayerState|GetPlayerName _asbp_moba_player_state))
              (Class|TeamComponent|SetTeam (Variables|/Script/MobaDegree.MobaPlayerState|GetTeamComponent _asbp_moba_player_state) "Blue")
              (Development|PrintString "BLUE" true true "(R=0.000000,G=0.861000,B=1.000000,A=1.000000)")
              (return)))
          (:Completed
            (return)))))))